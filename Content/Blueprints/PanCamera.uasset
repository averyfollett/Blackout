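; PanCamera is a camera actor that makes itself the player's view target and glides to a fixed offset from its start position.
; BeginPlay stores that target location, and Tick reasserts the view target while lerping toward it by Speed each frame, unscaled by delta time, until within tolerance.
; Rotation easing is unwired: TargetRotation is stored but unused, and the move call leaves its rotation input unset.
; Debug strings print on creation and movement.
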(event `self.ReceiveBeginPlay`
  ;[1 1 1] Set default camera location
  (`PlayerController.SetViewTargetWithBlend` (`GameplayStatics.GetPlayerController` 0) self 0.0 "VTBlend_Linear" 0.0 false)
  (set `self.TargetLocation` (+ (`self.K2_GetActorLocation`) (0.0 200.0 100.0)))
  (set `self.TargetRotation` (`self.K2_GetActorRotation`))
  (`KismetSystemLibrary.PrintString` "Created" true true (struct :`R` 0.912325 :`B` 1.0 :`A` 1.0) 6.0))

(event `self.ReceiveTick`
  (params (DeltaSeconds :type "Float (single-precision)"))
  (bind _returnvalue (`self.K2_GetActorLocation`))
  (bind _targetlocation (`self.TargetLocation`))
  ;[1 1 1] move camera to new target location
  (`PlayerController.SetViewTargetWithBlend` (`GameplayStatics.GetPlayerController` 0) self 0.0 "VTBlend_Linear" 0.0 false)
  (if (not (== _targetlocation _returnvalue :`ErrorTolerance` 0.1))
    (`self.K2_SetActorLocationAndRotation` (`KismetMathLibrary.VLerp` _returnvalue _targetlocation (`self.Speed`)))
    (`KismetSystemLibrary.PrintString` "Setting Camera Location")))

(fn `UserConstructionScript`)