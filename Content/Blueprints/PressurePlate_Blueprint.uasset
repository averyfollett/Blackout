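; Pressure plate that third-person characters press by standing on it, passing power to linked powerable actors.
; Overlaps track who is on it, drive a timeline that moves the top cube, and turn both dynamic materials green when pressed or red when released.
; StaysPressed latches it after the last character leaves.
; After a delay, it sends pressed AND powered to each NextPowerable, tagged with its own GUID as setter.
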(event `AnimatePressurePlate`
  ;[1 1 1] animate
  (bind (_direction _newtrack_0) (`Timeline|Timeline_0` :!label _label)
    (:`Update`
      (`SceneComponent.K2_SetRelativeLocation` (`self.Cube`) (`KismetMathLibrary.VLerp` (`self.PressurePlateStart`) (`self.PressurePlateEnd`) _newtrack_0) false false))))

(event `AnimateUnpressed`
  ;[1 1 1] animate
  (goto _label))

(event `self.ReceiveActorBeginOverlap`
  (params (OtherActor :type "Actor Object Reference"))
  ;[1 1 1] Press Pressure Plate
  (cast `/Game/Blueprints/ThirdPersonBP/Blueprints/ThirdPersonCharacter` OtherActor)
  (set `self.IsPressed` true)
  (`BlueprintSetLibrary.Set_Add` (`self.currentlyPressedBy`) OtherActor)
  (`self.Set Powered` (`self.isPowered`))
  (`self.AnimatePressurePlate`)
  (`self.Change To Green`))

(event `Change To Green`
  ;[1 1 1] Change Colors
  (`MaterialInstanceDynamic.SetVectorParameterValue` (`self.bottomMaterial`) "Emissive Color" (`KismetMathLibrary.MakeColor` 0.0 1.0))
  (`MaterialInstanceDynamic.SetVectorParameterValue` (`self.topMaterial`) "Emissive Color" (`KismetMathLibrary.MakeColor` 0.0 1.0)))

(event `self.ReceiveActorEndOverlap`
  (params (OtherActor :type "Actor Object Reference"))
  (bind _currentlypressedby (`self.currentlyPressedBy`))
  ;[1 1 1] Set end pressed
  (if (`BlueprintSetLibrary.Set_Contains` (`self.currentlyPressedBy`) OtherActor)
    (`BlueprintSetLibrary.Set_Remove` _currentlypressedby OtherActor)
    (if (== (`BlueprintSetLibrary.Set_Length` _currentlypressedby) 0)
      (if (`self.StaysPressed`)
        (set `self.IsPressed` true)
        (`self.Set Powered` (`self.isPowered`))
        (else
          (set `self.IsPressed` false)
          (`KismetSystemLibrary.PrintString` "Stays pressed false. ")
          (`self.Set Powered` (`self.isPowered`))
          (`self.AnimateUnpressed`)
          (`self.Change To Red`))))))

(event `Change To Red`
  ;[1 1 1] Change Colors
  (`MaterialInstanceDynamic.SetVectorParameterValue` (`self.bottomMaterial`) "Emissive Color" (`KismetMathLibrary.MakeColor` 1.0))
  (`MaterialInstanceDynamic.SetVectorParameterValue` (`self.topMaterial`) "Emissive Color" (`KismetMathLibrary.MakeColor` 1.0)))

(event `self.Set Powered`
  (params (isPowered :type Boolean) (setterID :type "Guid Structure"))
  ;[1 1 1] Set is powered
  (set `self.isPowered` isPowered)
  (`KismetSystemLibrary.Delay` (`self.Delay`))
  (`self.Set Next Powered` (and (`self.IsPressed`) isPowered)))

(event `Set Next Powered`
  (params (isPowered :type Boolean))
  ;[1 1 1] Set power state of nexts
  (for _array_element (`self.NextPowerables`)
    (message `/Game/Blueprints/WireElements/Powerable.Set Powered` _array_element isPowered (`self.thisGUID`))))

(event `self.ReceiveBeginPlay`
  ;[1 1 1] Inital Set up
  (bind _returnvalue (`PrimitiveComponent.CreateDynamicMaterialInstance` (`self.Cube1`) 0 null "None"))
  (set `self.bottomMaterial` _returnvalue)
  (bind _returnvalue_2 (`PrimitiveComponent.CreateDynamicMaterialInstance` (`self.Cube`) 0 null "None"))
  (set `self.topMaterial` _returnvalue_2)
  (set `self.thisGUID` (`KismetGuidLibrary.NewGuid`))
  (`self.Set Next Powered` (and (`self.isPowered`) (`self.IsPressed`))))

(fn `Get GUID`
  (returns (GUID :type "Guid Structure"))
  (return (`self.thisGUID`)))

(fn `UserConstructionScript`)