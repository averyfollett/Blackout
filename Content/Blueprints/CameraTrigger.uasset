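; CameraTrigger is an actor that repositions the camera when a ThirdPersonCharacter overlaps it.
; On overlap it passes the location of its PlaceholderCamera reference to the character's SetCamera and prints the controlled pawn's name as debug output.
; BeginPlay caches the first PanCamera actor in the level, though the overlap logic never uses it.
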(event `self.ReceiveBeginPlay`
  (bind _outactors (`GameplayStatics.GetAllActorsOfClass` "/Game/Blueprints/PanCamera.PanCamera_C"))
  (set `self.Pan Camera` (`|GetArrayItem` _outactors)))

(event `self.ReceiveActorBeginOverlap`
  (params (OtherActor :type "Actor Object Reference"))
  (bind _asthird_person_character (cast `/Game/Blueprints/ThirdPersonBP/Blueprints/ThirdPersonCharacter` OtherActor))
  (`/Game/Blueprints/ThirdPersonBP/Blueprints/ThirdPersonCharacter.Set Camera` _asthird_person_character (`self.K2_GetActorLocation` (`self.PlaceholderCamera`)))
  (`KismetSystemLibrary.PrintString` (`KismetSystemLibrary.GetDisplayName` (`Controller.K2_GetPawn` (`GameplayStatics.GetPlayerController` 0)))))

(fn `UserConstructionScript`)