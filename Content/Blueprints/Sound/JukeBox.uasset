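; JukeBox is a music player Blueprint that starts an attached audio event and adapts it to the current level.
; On BeginPlay it plays the Music event on its AudioComponent and sets the "Level" parameter from the map name, for Level_1 through Level_3.
; A ChangeMusic event passes CurrentPowerLevel to a parameter on AudioComponent, with no parameter name specified, rather than on the instance returned at BeginPlay.
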(event `self.ReceiveBeginPlay`
  (bind _returnvalue (`FMODBlueprintStatics.PlayEventAttached` "/Game/FMOD/Events/Music.Music" (`self.AudioComponent`) "None" (0.0 0.0 0.0) "KeepRelativeOffset"))
  (bind _returnvalue_2 (`GameplayStatics.GetCurrentLevelName` true))
  (if (`KismetStringLibrary.EqualEqual_StrStr` _returnvalue_2 "Level_1")
    (`FMODAudioComponent.SetParameter` _returnvalue "Level" 1.0)
    (elif (`KismetStringLibrary.EqualEqual_StrStr` _returnvalue_2 "Level_2")
      (`FMODAudioComponent.SetParameter` _returnvalue "Level" 2.0)
      (elif (`KismetStringLibrary.EqualEqual_StrStr` _returnvalue_2 "Level_3")
        (`FMODAudioComponent.SetParameter` _returnvalue "Level" 2.8)))))

(event `ChangeMusic`
  (`FMODAudioComponent.SetParameter` (`self.AudioComponent`) "PowerLevel" (`self.CurrentPowerLevel`)))

(fn `UserConstructionScript`)