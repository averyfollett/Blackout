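; Wire segment for a power-routing puzzle, toggled between Rotated and Unrotated states when something overlaps its box while powered or marked first.
; A FlipFlop sets the state flags without moving the actor, and Tick sets a blue or red emissive material from them.
; The first segment powers itself on BeginPlay.
; Logic passing power to NextRotated or NextUnrotated is disconnected, leaving HandlePowerOutput empty.
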(event `self.ReceiveTick`
  (params (DeltaSeconds :type "Float (single-precision)"))
  (`self.HandlePowerOutput`)
  (`self.HandleMaterialChange`))

(event `HandleMaterialChange`
  (if (`self.Rotated`)
    (`PrimitiveComponent.SetMaterial` (`self.StaticMeshComponent`) 0 "/Game/Assets/Materials/TempMat/MI_Grate_EmissiveBlue.MI_Grate_EmissiveBlue")
    (elif (`self.Unrotated`)
      (`PrimitiveComponent.SetMaterial` (`self.StaticMeshComponent`) 0 "/Game/Assets/Materials/TempMat/MI_Grate_EmissiveRed.MI_Grate_EmissiveRed"))))

(event `self.Box.OnComponentBeginOverlap`
  (params (OverlappedComponent :type "PrimitiveComponent Object Reference") (OtherActor :type "Actor Object Reference") (OtherComp :type "PrimitiveComponent Object Reference") (OtherBodyIndex :type Integer) (bFromSweep :type Boolean) (SweepResult :type "HitResult Structure (by ref)"))
  ;[1 1 1] rotate if powered
  (if (or (`self.IncomingPower`) (`self.IsFirst`))
    (`self.RotateWire`)
    (set `self.IncomingPower` true)))

(event `RotateWire`
  ;[1 1 1] rotate if powered
  (`/Engine/EditorBlueprintResources/StandardMacros.FlipFlop`
    (:`A`
      (set `self.Rotated` true)
      (set `self.Unrotated` false))
    (:`B`
      (set `self.Unrotated` true)
      (set `self.Rotated` false))))

(event `HandlePowerOutput`)

(event `self.ReceiveBeginPlay`
  (if (`self.IsFirst`)
    (set `self.IncomingPower` true)))

(fn `UserConstructionScript`)