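; Trigger actor that detects whether a pipe or wire piece (Pipe_Blueprint) has been placed on it.
; Actor begin and end overlap events compare the other actor's class to Pipe_Blueprint for an exact match, setting or clearing the IsPlaced flag.
; Debug strings print on every begin overlap and again when a pipe is placed; the construction script is empty.
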(event `self.ReceiveActorBeginOverlap`
  (params (OtherActor :type "Actor Object Reference"))
  (`KismetSystemLibrary.PrintString` "Something Collided")
  (if (== (`GameplayStatics.GetObjectClass` OtherActor) "/Game/Blueprints/Old/TutorialLevelBeta/Pipe_Blueprint.Pipe_Blueprint_C")
    (set `self.IsPlaced` true)
    (`KismetSystemLibrary.PrintString` "Pipe/Wire is placed")))

(event `self.ReceiveActorEndOverlap`
  (params (OtherActor :type "Actor Object Reference"))
  (if (== (`GameplayStatics.GetObjectClass` OtherActor) "/Game/Blueprints/Old/TutorialLevelBeta/Pipe_Blueprint.Pipe_Blueprint_C")
    (set `self.IsPlaced` false)))

(fn `UserConstructionScript`)