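; Wire-element trim that lights its emissive material when powered and relays that power along a chain.
; SetPowered stores each setter's state by ID and ANDs them all, with StayPowered optionally latching it on once powered.
; The result drives Emission on a dynamic material instance in slot 1, then passes to NextPowerables via SetPoweredMessage after PowerDelay.
; BeginPlay creates that material and sends an unpowered state downstream.
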(event `self.ReceiveBeginPlay`
  ;[1 1 1] Beginning Set up
  (set `self.thisGuid` (struct))
  (bind _returnvalue (`KismetMaterialLibrary.CreateDynamicMaterialInstance` "/Game/Assets/Materials/MI_emissiveTrimMaterial_00.MI_emissiveTrimMaterial_00"))
  (set `self.dynamicMaterialInstance` _returnvalue)
  (`self.Set Apperance` false)
  (`self.Power Nexts` false)
  (set `self.hasFinishedSetup` true))

(event `/Game/Blueprints/WireElements/Powerable.Set Powered`
  (params (isPowered :type Boolean) (setterID :type "Guid Structure"))
  (bind _isthispowered (`self.isThisPowered`))
  (bind _powerstateofinputs (`self.powerStateOfInputs`))
  ;[1 1 1] Set power state
  (`BlueprintMapLibrary.Map_Add` _powerstateofinputs setterID isPowered) ; Add this key to the map or reset its existing value
  (bind _values (`BlueprintMapLibrary.Map_Values` _powerstateofinputs))
  ;;[0.5776 0.6025 1] Set isThisPowered to first item in list
  (set `self.isThisPowered` (`|GetArrayItem` _values))
  ;;[1 0.1442 0.5712] Check if every item in array is true
  (for _array_element _values
    (set `self.isThisPowered` (and _array_element (`self.isThisPowered`))))
  (set `self.isThisPowered` (or (and (`self.stayPowered`) (`self.wasPowered`)) (`self.isThisPowered`)))
  ;;[0.3598 1 0.7041] Do things based on outcome
  (`self.Set Apperance` (`self.isThisPowered`))
  (`KismetSystemLibrary.Delay` (`self.PowerDelay`))
  (`self.Power Nexts` _isthispowered)
  (set `self.wasPowered` (or (`self.wasPowered`) _isthispowered)))

(event `Set Apperance`
  (params (isPowered :type Boolean))
  (bind _dynamicmaterialinstance (`self.dynamicMaterialInstance`))
  ;[1 1 1] Set Apperance
  (if (`self.hasFinishedSetup`)
    (`MaterialInstanceDynamic.SetScalarParameterValue` _dynamicmaterialinstance "Emission" (* (`KismetMathLibrary.Conv_BoolToDouble` isPowered) 50.0))
    (`PrimitiveComponent.SetMaterial` (`self.StaticMeshComponent`) 1 _dynamicmaterialinstance)))

(event `Power Nexts`
  (params (PowerState :type Boolean))
  ;[1 1 1] Power Next
  (for _array_element (`self.NextPowerables`)
    (message `/Game/Blueprints/WireElements/Powerable.Set Powered` _array_element PowerState (struct))))

(fn `Get GUID`
  (returns (GUID :type "Guid Structure"))
  (return))

(fn `UserConstructionScript`)