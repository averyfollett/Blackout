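; Powerable OR gate Blueprint for wire-style power networks, outputting powered when any recorded input is powered.
; SetPowered stores each sender's state in a map keyed by ID, ORs the values, calls an empty appearance event, then waits a delay before propagating.
; PowerNext messages every NextPowerable with the gate's own GUID, created on BeginPlay when the initial state is also sent.
; The wire material swap is present but disconnected.
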(event `/Game/Blueprints/WireElements/Powerable.Set Powered`
  (params (isPowered :type Boolean) (setterID :type "Guid Structure"))
  ;[1 1 1] Set power state
  (`BlueprintMapLibrary.Map_Add` (`self.powerStateOfInputs`) setterID isPowered)
  (bind _values (`BlueprintMapLibrary.Map_Values` (`self.powerStateOfInputs`)))
  (set `self.wasPowered` (`|GetArrayItem` _values))
  (for _array_element _values
    (set `self.wasPowered` (or _array_element (`self.wasPowered`))))
  (`self.Set Apperance` (`self.wasPowered`))
  (`KismetSystemLibrary.Delay` (`self.delay`))
  (`self.Power Next` (`self.wasPowered`)))

(event `self.ReceiveBeginPlay`
  ;[1 1 1] Begain Play
  (set `self.thisGuid` (`KismetGuidLibrary.NewGuid`))
  (`self.Power Next` (`self.wasPowered`)))

(event `Set Apperance`
  (params (isPowered :type Boolean))
  ;[1 1 1] Set apperance
)

(event `Power Next`
  (params (isPowered :type Boolean))
  ;[1 1 1] Power Next
  (for _array_element (`self.NextPowerables`)
    (message `/Game/Blueprints/WireElements/Powerable.Set Powered` _array_element isPowered (`self.thisGuid`))))

(fn `Get GUID`
  (returns (GUID :type "Guid Structure"))
  (return))

(fn `UserConstructionScript`)