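; Spline-based wire actor that shows power flowing along it and passes that power state on to connected powerable objects.
; The construction script builds a spline mesh per spline segment, and BeginPlay gives each a dynamic material and a unique GUID for the wire.
; Power changes toggle the "On/Off" material parameter segment by segment with a delay, in the direction set by IsFoward.
; SetPowerNext forwards the state and GUID to each NextPowerable.
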(event `self.ReceiveBeginPlay`
  (bind _ispowered (`self.isPowered`))
  ;[1 1 1] Begin Play: Set ID and apperance
  (set `self.thisGuid` (`KismetGuidLibrary.NewGuid`))
  (for _array_element (`self.SplineMeshes`)
    (bind _returnvalue (`KismetMaterialLibrary.CreateDynamicMaterialInstance` (`PrimitiveComponent.GetMaterial` _array_element 0)))
    (`KismetArrayLibrary.Array_Add` (`self.dynamicMaterials`) _returnvalue))
  (set `self.isSetupDone` true)
  (`self.SetApperance` _ispowered)
  (`self.Set Power Next` _ispowered))

(event `/Game/Blueprints/WireElements/Powerable.Set Powered`
  (params (isPowered :type Boolean) (setterID :type "Guid Structure"))
  ;[1 1 1] Set is powered
  (bind _output_get (set `self.isPowered` isPowered))
  (`self.SetApperance` isPowered)
  (`KismetSystemLibrary.Delay` (`self.Set Next Delay`))
  (`self.Set Power Next` _output_get))

(event `SetApperance`
  (params (isPowered :type Boolean))
  (bind _splinemeshes (`self.SplineMeshes`))
  (bind _splinemeshes_2 (`self.SplineMeshes`))
  (bind _i (`self.i`))
  (bind _i_2 (`self.i`))
  ;[1 1 1] Set material based on power state
  (if (`self.isSetupDone`)
    (if (`self.isFoward`)
      ;;[1 1 1] Light up wire in one derection
      (set `self.i` (- (`KismetArrayLibrary.Array_Length` _splinemeshes_2) 1))
      (if (>= (`self.i`) 0) :!label _label
        (bind _output_get (set `self.currentMaterial` (`|GetArrayItem` (`self.dynamicMaterials`) _i)))
        (`MaterialInstanceDynamic.SetScalarParameterValue` _output_get "On/Off" (`KismetMathLibrary.Conv_BoolToDouble` isPowered))
        (`PrimitiveComponent.SetMaterial` (`|GetArrayItem` _splinemeshes_2 _i) 0 _output_get)
        (set `self.i` (- (`self.i`) 1))
        (`KismetSystemLibrary.Delay` (`self.Set Next Delay`))
        (goto _label))
      (else
        ;;[1 1 1] Light up wire other derection
        (set `self.i` 0)
        (if (< (`self.i`) (`KismetArrayLibrary.Array_Length` _splinemeshes)) :!label _label_2
          (bind _output_get_2 (set `self.currentMaterial` (`|GetArrayItem` (`self.dynamicMaterials`) _i_2)))
          (`MaterialInstanceDynamic.SetScalarParameterValue` _output_get_2 "On/Off" (`KismetMathLibrary.Conv_BoolToDouble` isPowered))
          (`PrimitiveComponent.SetMaterial` (`|GetArrayItem` _splinemeshes _i_2) 0 _output_get_2)
          (set `self.i` (+ (`self.i`) 1))
          (`KismetSystemLibrary.Delay` (`self.Set Next Delay`))
          (goto _label_2))))))

(event `Set Power Next`
  (params (isPowered :type Boolean))
  ;[1 1 1] Set power state of next connection
  (for _array_element (`self.NextPowerable`)
    (message `/Game/Blueprints/WireElements/Powerable.Set Powered` _array_element isPowered (`self.thisGuid`))))

(fn `Get GUID`
  (returns (GUID :type "Guid Structure"))
  (return (`self.thisGuid`)))

(fn `UserConstructionScript`
  (for _index (range (+ (- (`SplineComponent.GetNumberOfSplinePoints` (`self.Spline1`)) 2) 1))
    (bind _returnvalue (`AddComponent|NODE_AddSplineMeshComponent-1`))
    (`KismetArrayLibrary.Array_Add` (`self.SplineMeshes`) _returnvalue)
    (`SplineMeshComponent.SetForwardAxis` _returnvalue "Z" true)
    (`self.K2_AttachToComponent` (`self.Spline1`) "None" "KeepRelative" "KeepRelative" "KeepRelative")
    (bind (_location _tangent) (`SplineComponent.GetLocationAndTangentAtSplinePoint` (`self.Spline1`) _index "Local"))
    (bind (_location_2 _tangent_2) (`SplineComponent.GetLocationAndTangentAtSplinePoint` (`self.Spline1`) (+ _index 1) "Local"))
    (`SplineMeshComponent.SetStartAndEnd` _returnvalue _location _tangent _location_2 _tangent_2 true)))