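; SplineTrim is a wire element actor that builds a run of deformed mesh along an editable spline.
; The construction script adds one spline mesh component per segment, attaches it to Spline1 and stores it in SplineMeshes.
; Each segment takes its start and end from adjacent points' local locations and tangents, with Z as the forward axis.
; A Get GUID function returns the stored ThisGuid identifier.
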(fn `Get GUID`
  (returns (GUID :type "Guid Structure"))
  (return (`self.thisGuid`)))

(fn `UserConstructionScript`
  (for _index (range (+ (- (`SplineComponent.GetNumberOfSplinePoints` (`self.Spline1`)) 2) 1))
    (bind _returnvalue (`AddComponent|NODE_AddSplineMeshComponent-1`))
    (`KismetArrayLibrary.Array_Add` (`self.SplineMeshes`) _returnvalue)
    (`SplineMeshComponent.SetForwardAxis` _returnvalue "Z" true)
    (`self.K2_AttachToComponent` (`self.Spline1`) "None" "KeepRelative" "KeepRelative" "KeepRelative")
    (bind (_location _tangent) (`SplineComponent.GetLocationAndTangentAtSplinePoint` (`self.Spline1`) _index "Local"))
    (bind (_location_2 _tangent_2) (`SplineComponent.GetLocationAndTangentAtSplinePoint` (`self.Spline1`) (+ _index 1) "Local"))
    (`SplineMeshComponent.SetStartAndEnd` _returnvalue _location _tangent _location_2 _tangent_2 true)))