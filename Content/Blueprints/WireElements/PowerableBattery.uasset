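; PowerableBattery is a wire-element Blueprint that holds a power state and passes it to connected powerable elements.
; On BeginPlay it creates a GUID and dynamic material, then shows green or red emissive for its state.
; It sends that state to each NextPowerable with its GUID as setter ID.
; SetPowered acts only on a true value, so it never switches the battery off.
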(event `self.ReceiveBeginPlay`
  ;[1 1 1] Begin Play: Set ID and apperance
  (set `self.thisGuid` (`KismetGuidLibrary.NewGuid`))
  (bind _returnvalue (`PrimitiveComponent.CreateDynamicMaterialInstance` (`self.StaticMeshComponent`) 0 null "None"))
  (set `self.dynamicMaterialInstance` _returnvalue)
  (set `self.setupDone` true)
  (`self.SetApperance`)
  (`self.Set Power Next` (`self.isPowered`)))

(event `/Game/Blueprints/WireElements/Powerable.Set Powered`
  (params (isPowered :type Boolean) (setterID :type "Guid Structure"))
  ;[1 1 1] Set is powered
  (if isPowered
    (set `self.isPowered` isPowered)
    (`self.SetApperance`)
    (`self.Set Power Next` isPowered)))

(event `SetApperance`
  (bind _dynamicmaterialinstance (`self.dynamicMaterialInstance`))
  ;[1 1 1] Set material based on power state
  (if (`self.setupDone`)
    (if (`self.isPowered`)
      (`MaterialInstanceDynamic.SetVectorParameterValue` _dynamicmaterialinstance "Emissive Color" (`KismetMathLibrary.MakeColor` 0.0 1.0))
      (else
        (`MaterialInstanceDynamic.SetVectorParameterValue` _dynamicmaterialinstance "Emissive Color" (`KismetMathLibrary.MakeColor` 1.0 0.0))))))

(event `Set Power Next`
  (params (isPowered :type Boolean))
  ;[1 1 1] Set power state of next connection
  (for _array_element (`self.NextPowerable`)
    (message `/Game/Blueprints/WireElements/Powerable.Set Powered` _array_element isPowered (`self.thisGuid`))))

(fn `Get GUID`
  (returns (GUID :type "Guid Structure"))
  (return (`self.thisGuid`)))

(fn `UserConstructionScript`)