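; Wire element Blueprint that relays a powered state to connected powerable objects in a circuit.
; On BeginPlay it creates a GUID and a dynamic material, then pushes its initial power state onward.
; SetPowered updates the material's On/Off parameter, waits SetNextDelay, then messages each NextPowerable with the state and its GUID as setter ID, giving staggered propagation.
; SetupDone is set last, so the initial appearance update is skipped.
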(event `self.ReceiveBeginPlay`
  ;[1 1 1] Begin Play: Set ID and apperance
  (set `self.thisGuid` (`KismetGuidLibrary.NewGuid`))
  (bind _returnvalue (`KismetMaterialLibrary.CreateDynamicMaterialInstance` (`PrimitiveComponent.GetMaterial` (`self.StaticMeshComponent`) 0)))
  (set `self.Dynamic Material Instance` _returnvalue)
  (`self.SetApperance`)
  (`self.Set Power Next` (`self.isPowered`))
  (set `self.setupDone` true))

(event `/Game/Blueprints/WireElements/Powerable.Set Powered`
  (params (isPowered :type Boolean) (setterID :type "Guid Structure"))
  ;[1 1 1] Set is powered
  (bind _output_get (set `self.isPowered` isPowered))
  (`self.SetApperance`)
  (`KismetSystemLibrary.Delay` (`self.Set Next Delay`))
  (`self.Set Power Next` _output_get))

(event `SetApperance`
  (bind _dynamic_material_instance (`self.Dynamic Material Instance`))
  ;[1 1 1] Set material based on power state
  (if (`self.setupDone`)
    (`MaterialInstanceDynamic.SetScalarParameterValue` _dynamic_material_instance "On/Off" (`KismetMathLibrary.Conv_BoolToDouble` (`self.isPowered`)))
    (`PrimitiveComponent.SetMaterial` (`self.StaticMeshComponent`) 0 _dynamic_material_instance)))

(event `Set Power Next`
  (params (isPowered :type Boolean))
  ;[1 1 1] Set power state of next connection
  (for _array_element (`self.NextPowerable`)
    (message `/Game/Blueprints/WireElements/Powerable.Set Powered` _array_element isPowered (`self.thisGuid`))))

(fn `Get GUID`
  (returns (GUID :type "Guid Structure"))
  (return (`self.thisGuid`)))

(fn `UserConstructionScript`)