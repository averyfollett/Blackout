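; PowerableObjects is a base Blueprint for wire elements that can be switched between powered and unpowered.
; SetPowered updates the appearance, waits for a Delay, then calls SetNext with the same state, allowing staggered propagation.
; SetApperance and SetNext are placeholders that only print base-class messages, apparently for child classes to override.
; BeginPlay stores a new GUID and prints a message, while GetGUID returns without a connected value.
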(event `/Game/Blueprints/WireElements/Powerable.Set Powered`
  (params (isPowered :type Boolean) (setterID :type "Guid Structure"))
  (`self.Set Apperance` isPowered)
  (`KismetSystemLibrary.Delay` (`self.delay`))
  (`self.Set Next` isPowered))

(event `self.ReceiveBeginPlay`
  (set `self.thisGuid` (`KismetGuidLibrary.NewGuid`))
  (`KismetSystemLibrary.PrintString` "Calling base class Event Begin Play"))

(event `Set Next`
  (params (isPowered :type Boolean))
  (`KismetSystemLibrary.PrintString` "Calling base class set next"))

(event `Set Apperance`
  (params (`is it powered` :type Boolean))
  (`KismetSystemLibrary.PrintString` "Calling base class set apperance"))

(fn `Get GUID`
  (returns (GUID :type "Guid Structure"))
  (return))

(fn `UserConstructionScript`)