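; Powered lift actor that moves its Lift component between a start and end location when switched on through SetPowered.
; LoopMovement selects either a looping timeline, which stops looping on power loss to finish its run, or a one-way timeline that reverses.
; A 2D sound event plays while powered and stops on power loss.
; A GUID generated at BeginPlay is exposed through GetGUID.
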(event `PowerLift`
  ;[1 1 1] lift movement
  (bind _returnvalue (`FMODBlueprintStatics.PlayEvent2D` "/Game/FMOD/Events/Env/Lift.Lift"))
  (if (`self.LoopMovement`)
    (`TimelineComponent.SetLooping` (`self.LiftMovementTimeline`) true)
    (bind (_direction _driver) (`Timeline|LiftMovementTimeline`)
      (:`Update`
        (`SceneComponent.K2_SetRelativeLocation` (`self.Lift`) (`KismetMathLibrary.VLerp` (`self.LiftStart`) (`self.LiftEnd`) _driver) false false)))
    (else
      (bind (_direction_2 _driver_2) (`Timeline|LiftMovementTimelineNotLooping` :!label _label)
        (:`Update`
          (`SceneComponent.K2_SetRelativeLocation` (`self.Lift`) (`KismetMathLibrary.VLerp` (`self.LiftStart`) (`self.LiftEnd`) _driver_2) false false))))))

(event `UnpowerLift`
  ;[1 1 1] lift movement
  (`FMODBlueprintStatics.EventInstanceStop` (stale `PowerLift` _returnvalue) true)
  (if (`self.LoopMovement`)
    (`TimelineComponent.SetLooping` (`self.LiftMovementTimeline`) false)
    (else
      (goto _label :!via `Reverse`))))

(event `self.ReceiveBeginPlay`
  ;[1 1 1] Guid
  (set `self.thisGuid` (`KismetGuidLibrary.NewGuid`)))

(event `/Game/Blueprints/WireElements/Powerable.Set Powered`
  (params (isPowered :type Boolean) (setterID :type "Guid Structure"))
  ;[1 1 1] Set powered
  (if isPowered
    (`self.PowerLift`)
    (else
      (`self.UnpowerLift`))))

(fn `Get GUID`
  (returns (GUID :type "Guid Structure"))
  (return (`self.thisGuid`)))

(fn `UserConstructionScript`)