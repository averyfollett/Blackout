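; Powered turret that launches Player-tagged pawns away from itself, showing power state through green/red materials, an effect and sound.
; SetPowered runs a looping sphere-trace scan that acquires a target; overlapping ViewArea also calls LaunchPlayer on any Character while powered.
; Older tracking logic (line-of-sight, yaw-clamped head rotation, launch when aligned) sits behind a gate that is opened but never entered, as Tick is empty.
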(event `Set Apperance`
  (params (isPowered :type Boolean))
  (bind _returnvalue (`KismetMathLibrary.MakeColor` 1.0))
  (bind _returnvalue_2 (`KismetMathLibrary.MakeColor` 0.0 1.0))
  (bind _turretbasematerial (`self.turretBaseMaterial`))
  ;[1 1 1] Set apperance
  (if isPowered
    ;[1 1 1] Change Color to Green
    (`MaterialInstanceDynamic.SetVectorParameterValue` (`self.turretBaseMaterial`) "Emissive Color" _returnvalue_2)
    (`MaterialInstanceDynamic.SetVectorParameterValue` (`self.turretHeadMaterial`) "Emissive Color" _returnvalue_2)
    (`KismetSystemLibrary.PrintString` "TODO: Set turret apperance")
    (`ActorComponent.Activate` (`self.PS_PSHHH`) false)
    (else
      ;[1 1 1] Change Color to Red (errors should be fixed)
      (`/Engine/EditorBlueprintResources/StandardMacros.IsValid` _turretbasematerial
        (:`Is Valid`
          (`MaterialInstanceDynamic.SetVectorParameterValue` _turretbasematerial "Emissive Color" _returnvalue)
          (`MaterialInstanceDynamic.SetVectorParameterValue` (`self.turretHeadMaterial`) "Emissive Color" _returnvalue)
          (`ActorComponent.Deactivate` (`self.PS_PSHHH`)))))))

(event `/Game/Blueprints/WireElements/Powerable.Set Powered`
  (params (isPowered :type Boolean) (setterID :type "Guid Structure"))
  ;[1 1 1] Set powered
  (set `self.Powered` isPowered)
  (`self.Set Apperance` isPowered)
  (if isPowered
    (`KismetSystemLibrary.K2_SetTimer` self "ScanForTargetTimer" 0.2 true)
    (`/Engine/EditorBlueprintResources/StandardMacros.DoOnce` false :!label _label
      (:`Completed`
        (`self.PlayTurning` false
          (:`End`
            (goto _label_2 :!via `Reset`)))))
    (else
      (`KismetSystemLibrary.K2_ClearTimer` self "ScanForTargetTimer")
      (`self.CloseFiringGate`)
      (`/Engine/EditorBlueprintResources/StandardMacros.DoOnce` false :!label _label_2
        (:`Completed`
          (`self.PlayTurning` true :!via `Stop`
            (:`End`
              (goto _label :!via `Reset`))))))))

(event `Launch Player`
  (params (targetActor :type "Actor Object Reference"))
  ;[1 1 1] Launch Target
  (if (`self.Powered`)
    (bind _ascharacter (cast `Character` targetActor))
    (`Character.LaunchCharacter` _ascharacter (+ (* (`KismetMathLibrary.Normal` (- (`self.K2_GetActorLocation` targetActor) (`self.K2_GetActorLocation`))) (`self.Strength`)) (`self.launchModifier`)) true true)
    (`/Engine/EditorBlueprintResources/StandardMacros.DoOnce` false :!label _label_3
      (:`Completed`
        (`FMODBlueprintStatics.PlayEvent2D` "/Game/FMOD/Events/Env/TurretShoot.TurretShoot")))
    (else
      (goto _label_3 :!via `Reset`))))

(event `self.ReceiveBeginPlay`
  ;[1 1 1] Beginning Set up
  ;[1 1 1] Create Dynamic Materials
  (bind _returnvalue (`PrimitiveComponent.CreateDynamicMaterialInstance` (`self.Base`) 0 null "None"))
  (set `self.turretBaseMaterial` _returnvalue)
  (bind _returnvalue_2 (`PrimitiveComponent.CreateDynamicMaterialInstance` (`self.SM_turretTop_01`) 0 null "None"))
  (set `self.turretHeadMaterial` _returnvalue_2)
  (set `self.thisGuid` (`KismetGuidLibrary.NewGuid`))
  (if (`self.Powered`)
    _))

(event `self.ViewArea.OnComponentBeginOverlap`
  (params (OverlappedComponent :type "PrimitiveComponent Object Reference") (OtherActor :type "Actor Object Reference") (OtherComp :type "PrimitiveComponent Object Reference") (OtherBodyIndex :type Integer) (bFromSweep :type Boolean) (SweepResult :type "HitResult Structure (by ref)"))
  (`self.Launch Player` OtherActor))

(event `self.ReceiveTick`
  (params (DeltaSeconds :type "Float (single-precision)"))
  ;[1 0 0] OLD Turret Code
)

(event `ScanForTargetTimer`
  (bind _sm_turrettop_01 (`self.SM_turretTop_01`))
  (bind _target (`self.Target`))
  (bind _returnvalue (`SceneComponent.K2_GetComponentRotation` _sm_turrettop_01))
  (bind _returnvalue_2 (`KismetMathLibrary.FindLookAtRotation` (`SceneComponent.K2_GetComponentLocation` _sm_turrettop_01) (`self.K2_GetActorLocation` (`self.Target`))))
  (bind _yaw (.yaw _returnvalue_2))
  ;[1 0 0] OLD Turret Code
  (bind _outhit (`KismetSystemLibrary.SphereTraceSingleForObjects` :`Start` (`SceneComponent.K2_GetComponentLocation` (`self.SM_turretTop_01`)) :`End` (`self.K2_GetActorLocation` self) :`Radius` (`self.ViewDistance`) :`ObjectTypes` (`|MakeArray` "ObjectTypeQuery3" :!type "EObjectTypeQuery Enum") :`DrawDebugType` "ForDuration"))
  (bind (_bblockinghit _binitialoverlap _time _distance _location _impactpoint _normal _impactnormal _physmat _hitactor) (`GameplayStatics.BreakHitResult` _outhit))
  (`/Engine/EditorBlueprintResources/StandardMacros.IsValid` _hitactor
    (:`Is Valid`
      (if (`self.ActorHasTag` _hitactor "Player")
        (`/Engine/EditorBlueprintResources/StandardMacros.IsValid` (`self.Target`)
          (:`Is Valid`
            (`/Engine/EditorBlueprintResources/StandardMacros.Gate` true :!via `Open` :!label _label_4
              (:`Exit`
                _)))
          (:`Is Not Valid`
            (set `self.Target` _hitactor)
            (goto _label_4 :!via `Open`)))
        (`/Engine/EditorBlueprintResources/StandardMacros.IsValid` _target
          (:`Is Valid`
            (bind _outhit_2 (`KismetSystemLibrary.LineTraceSingleForObjects` :`Start` (`SceneComponent.K2_GetComponentLocation` (`self.SM_turretTop_01`)) :`End` (`self.K2_GetActorLocation` _target) :`ObjectTypes` (`|MakeArray` "ObjectTypeQuery3" "ObjectTypeQuery1" :!type "EObjectTypeQuery Enum") :`DrawTime` 0.5))
            (bind (_bblockinghit_2 _binitialoverlap_2 _time_2 _distance_2 _location_2 _impactpoint_2 _normal_2 _impactnormal_2 _physmat_2 _hitactor_2) (`GameplayStatics.BreakHitResult` _outhit_2))
            (`/Engine/EditorBlueprintResources/StandardMacros.IsValid` _hitactor_2
              (:`Is Valid`
                (if (`self.ActorHasTag` _hitactor_2 "Player")
                  (if (<= (`self.GetDistanceTo` _hitactor_2 self) (`self.ViewDistance`))
                    (if (and (<= (`self.Max Angle`) _yaw) (>= _yaw (`self.Min Angle`)))
                      (`KismetSystemLibrary.PrintString` (`KismetStringLibrary.Conv_DoubleToString` _yaw))
                      (`SceneComponent.K2_SetWorldRotation` (`self.SM_turretTop_01`) (`KismetMathLibrary.MakeRotator` (.roll (`KismetMathLibrary.RInterpTo` _returnvalue _returnvalue_2 (`GameplayStatics.GetWorldDeltaSeconds`) (`self.RotationSpeed`))) (.pitch (`KismetMathLibrary.RInterpTo` _returnvalue _returnvalue_2 (`GameplayStatics.GetWorldDeltaSeconds`) (`self.RotationSpeed`))) (`KismetMathLibrary.ClampAngle` (.yaw (`KismetMathLibrary.RInterpTo` _returnvalue _returnvalue_2 (`GameplayStatics.GetWorldDeltaSeconds`) (`self.RotationSpeed`))) (`self.Min Angle`) (`self.Max Angle`))) false false)
                      (if (== _returnvalue _returnvalue_2 :`ErrorTolerance` 3.5)
                        (`/Engine/EditorBlueprintResources/StandardMacros.IsValid` _hitactor_2
                          (:`Is Valid`
                            (`self.Launch Player` (`self.Target`)))
                          (:`Is Not Valid`
                            (set `self.Target` null)))))
                    (else
                      (set `self.Target` null :!label _label_5)
                      (`self.CloseFiringGate`)))
                  (else
                    (goto _label_5)))))))))))

(event `CloseFiringGate`
  (bind _sm_turrettop_01 (`self.SM_turretTop_01`))
  ;[1 0 0] OLD Turret Code
  (`SceneComponent.K2_SetWorldRotation` _sm_turrettop_01 (`SceneComponent.K2_GetComponentRotation` _sm_turrettop_01) false false)
  (goto _label_4 :!via `Close`))

(fn `Get GUID`
  (returns (GUID :type "Guid Structure"))
  (return (`self.thisGuid`)))

(fn `UserConstructionScript`)