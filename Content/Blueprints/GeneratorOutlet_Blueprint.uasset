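; Generator outlet that powers linked lights and objects while a generator actor overlaps it.
; Overlap toggles light visibility and sends powered messages tagged with the outlet's GUID to each connected object, with StaysPressed optionally keeping power on after removal.
; A generator not being held snaps to the outlet's center with sparks and a timeline-driven yaw rotation.
; Generator noise unpauses and pauses on any actor's overlap, before the class check.
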(event `self.ReceiveBeginPlay`
  ;[1 1 1] Create new GUID
  (set `self.ThisGuid` (`KismetGuidLibrary.NewGuid`))
  (`FMODAudioComponent.SetPaused` (`self.GeneratorNoise1`) true))

(event `Set Lights Active`
  (params (isActive :type Boolean))
  ;[1 1 1] Set Lights
  (for _array_element (`self.lights`)
    (`SceneComponent.SetVisibility` (`Actor.RootComponent` _array_element) isActive false)))

(event `Set List Power State`
  (params (isPowered :type Boolean))
  ;[1 1 1] Set the power state of all connections
  (for _array_element (`self.PoweredObjects`)
    (message `/Game/Blueprints/WireElements/Powerable.Set Powered` _array_element isPowered (`self.ThisGuid`))))

(event `Snap to center`
  (params (Generator :type "/Game/Blueprints/Generator_Blueprint_New Object Reference"))
  (bind _returnvalue (+ (`self.K2_GetActorLocation`) (`KismetMathLibrary.MakeVector` 0.0 0.0 (`self.zOffset`))))
  ;[1 1 1] Snap to center
  (`KismetSystemLibrary.PrintString` "Snapping to center")
  (`self.K2_SetActorLocation` Generator _returnvalue false false)
  (`GameplayStatics.SpawnEmitterAtLocation` (`self.sparksParticles`) _returnvalue)
  (bind (_direction _zrotation) (`Timeline|rotateGenerator` :!via `PlayFromStart`)
    (:`Update`
      (`self.K2_SetActorRotation` Generator (`KismetMathLibrary.MakeRotator` 0.0 0.0 _zrotation) false))))

(event `self.ReceiveActorBeginOverlap`
  (params (OtherActor :type "Actor Object Reference"))
  ;[1 1 1] Generator Placed
  (`FMODAudioComponent.SetPaused` (`self.GeneratorNoise1`) false)
  (if (== (`GameplayStatics.GetObjectClass` OtherActor) "/Game/Blueprints/Generator_Blueprint_New.Generator_Blueprint_New_C")
    (bind _output_get (set `self.IsPressed` true))
    (`self.Set Lights Active` _output_get)
    (`self.Set List Power State` _output_get)
    (bind _asgenerator_blueprint_new (cast `/Game/Blueprints/Generator_Blueprint_New` OtherActor))
    (if (not (`/Game/Blueprints/Generator_Blueprint_New.isHeld` _asgenerator_blueprint_new))
      (`self.Snap to center` _asgenerator_blueprint_new))))

(event `self.ReceiveActorEndOverlap`
  (params (OtherActor :type "Actor Object Reference"))
  ;[1 1 1] Generator Removed
  (`FMODAudioComponent.SetPaused` (`self.GeneratorNoise1`) true)
  (if (== (`GameplayStatics.GetObjectClass` OtherActor) "/Game/Blueprints/Generator_Blueprint_New.Generator_Blueprint_New_C")
    (if (not (`self.StaysPressed`))
      (bind _output_get (set `self.IsPressed` false))
      (`self.Set Lights Active` _output_get)
      (`self.Set List Power State` _output_get))))

(fn `UserConstructionScript`)