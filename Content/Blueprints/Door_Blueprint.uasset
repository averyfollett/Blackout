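; Door actor that opens when it receives power, with no handling for losing power.
; SetPowered prints a debug message, disables the actor's collision and calls MoveDoor.
; MoveDoor plays a timeline that lerps the Door component between start and end locations, calling ActivateLights on every update to make the referenced lights visible.
; GetGUID and the construction script are empty stubs.
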(event `/Game/Blueprints/WireElements/Powerable.Set Powered`
  (params (isPowered :type Boolean) (setterID :type "Guid Structure"))
  ;[1 1 1] Set door power state
  (if isPowered
    (`KismetSystemLibrary.PrintString` "Set powered for door")
    (`self.SetActorEnableCollision` false)
    (`self.Move Door`)))

(event `Move Door`
  ;[1 1 1] Actually Move the door
  (bind (_direction _driver) (`Timeline|DoorMovementTimeline`)
    (:`Update`
      (`SceneComponent.K2_SetRelativeLocation` (`self.Door`) (`KismetMathLibrary.VLerp` (`self.DoorStart`) (`self.DoorEnd`) _driver) false false)
      (`self.Activate Lights`))))

(event `Activate Lights`
  ;[1 1 1] Activate Lights
  (for _array_element (`self.lights`)
    (`SceneComponent.SetVisibility` (`Light.LightComponent` _array_element) true false)))

(fn `Get GUID`
  (returns (GUID :type "Guid Structure"))
  (return))

(fn `UserConstructionScript`)